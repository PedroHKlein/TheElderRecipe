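; Mandrake ingredient actor that adds itself to a cauldron when the two overlap.
; On overlap with a Cauldron_BP, it writes a fixed ingredient enum value into the first free of three slots, chosen by IngredientCount, and increments that count.
; It destroys itself once added, and stays in the world if the cauldron already holds three ingredients.
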(event `self.ReceiveActorBeginOverlap`
  (params (OtherActor :type "Actor Object Reference"))
  (cast `/Game/Blueprints/Cauldron_BP` OtherActor)
  (if true
    (bind _ascauldron_bp (cast `/Game/Blueprints/Cauldron_BP` OtherActor))
    (if (== (`/Game/Blueprints/Cauldron_BP.IngredientCount` _ascauldron_bp) 0)
      (set `/Game/Blueprints/Cauldron_BP.Ingredient_01` "NewEnumerator0" _ascauldron_bp)
      (set `/Game/Blueprints/Cauldron_BP.IngredientCount` 1 _ascauldron_bp)
      (`self.K2_DestroyActor` :!label _label)
      (elif (== (`/Game/Blueprints/Cauldron_BP.IngredientCount` _ascauldron_bp) 1)
        (set `/Game/Blueprints/Cauldron_BP.Ingredient_02` "NewEnumerator0" _ascauldron_bp)
        (set `/Game/Blueprints/Cauldron_BP.IngredientCount` 2 _ascauldron_bp)
        (goto _label)
        (elif (== (`/Game/Blueprints/Cauldron_BP.IngredientCount` _ascauldron_bp) 2)
          (set `/Game/Blueprints/Cauldron_BP.Ingredient_03` "NewEnumerator0" _ascauldron_bp)
          (set `/Game/Blueprints/Cauldron_BP.IngredientCount` 3 _ascauldron_bp)
          (goto _label))))))

(fn `UserConstructionScript`)