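; Cauldron actor that checks three ingredient slots and spawns either a cure-disease potion or a bad potion.
; Every Tick it counts the slots matching the same expected enum value, then resets the counter.
; Three matches spawn the good potion; anything less spawns the bad one, offset from the mesh.
; DoOnce limits each outcome to one spawn, though the bad branch fires on any incomplete tick.
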(event `self.ReceiveTick`
  (params (DeltaSeconds :type "Float (single-precision)"))
  (if (`|EnumEquality` (`self.Ingredient_01`) "NewEnumerator0")
    (set `self.IngredientCheck` (+ (`self.IngredientCheck`) 1))
    (else
      (set `self.IngredientCheck` (+ (`self.IngredientCheck`) 0))))
  (set `self.IngredientOrder` 1)
  (if (`|EnumEquality` (`self.Ingredient_02`) "NewEnumerator0")
    (set `self.IngredientCheck` (+ (`self.IngredientCheck`) 1))
    (else
      (set `self.IngredientCheck` (+ (`self.IngredientCheck`) 0))))
  (set `self.IngredientOrder` 2)
  (if (`|EnumEquality` (`self.Ingredient_03`) "NewEnumerator0")
    (set `self.IngredientCheck` (+ (`self.IngredientCheck`) 1))
    (else
      (set `self.IngredientCheck` (+ (`self.IngredientCheck`) 0))))
  (if (>= (`self.IngredientCheck`) 3)
    (`/Engine/EditorBlueprintResources/StandardMacros.DoOnce` false
      (:`Completed`
        (set `self.Good Potion` "NewEnumerator2")
        (`|SpawnActorFromClass` "/Game/Blueprints/PotionCureDisease_BP.PotionCureDisease_BP_C" (`KismetMathLibrary.MakeTransform` (+ (`SceneComponent.K2_GetComponentLocation` (`self.StaticMeshComponent`)) (-100.0 0.0 100.0))) "Undefined" "OverrideRootScale" null null)
        (`KismetSystemLibrary.PrintString` "GoodPotion")))
    (else
      (`/Engine/EditorBlueprintResources/StandardMacros.DoOnce` false
        (:`Completed`
          (set `self.Bad Potion` "NewEnumerator0")
          (`|SpawnActorFromClass` "/Game/Blueprints/BadPotion_BP.BadPotion_BP_C" (`KismetMathLibrary.MakeTransform` (+ (`SceneComponent.K2_GetComponentLocation` (`self.StaticMeshComponent`)) (-100.0 0.0 100.0))) "Undefined" "OverrideRootScale" null null)
          (`KismetSystemLibrary.PrintString` "BadPotion")))))
  (set `self.IngredientOrder` 0)
  (set `self.IngredientCheck` 0))

(fn `UserConstructionScript`)